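; Enemy AI character that spots and attacks the player, and is defeated by any damage it takes.
; Pawn sensing sets the SeePlayer blackboard key and starts chase music, while a looping timer clears the key and fades the music if sight is not regained.
; AttackPlayer plays a shove montage, immediately sphere-tracing forward to apply damage.
; Taking damage ragdolls it, shows the win widget and plays sounds.
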(event OnSeePawn(PawnSensing)
  (params (Pawn :type Pawn%20Object%20Reference))
  (if (Actor|ActorHasTag Pawn "Player")
    (AI|Components|Blackboard|SetValueasBool (AI|GetBlackboard (AI|GetAIController self)) (Utilities|Name|MakeLiteralName "SeePlayer") true)
    (Variables|Default|GetChasing%20Music
      (:then)
      (:else
        (bind _returnvalue (Audio|SpawnSound2D "/Game/Audio/ScaryViolins.ScaryViolins" 1.0 1.0 0.0 0))
        (bind _output_get (Variables|Default|SetChasing%20Music _returnvalue))
        (Audio|Components|Audio|FadeIn _output_get 3.0 1.0 0.0 "Linear" :!class /Script/Engine.AudioComponent)))))

(event Custom|Attack%20Player
  (bind _attack_trace_point (Variables|Default|GetAttack%20Trace%20Point))
  (bind _returnvalue (Transformation|GetWorldLocation _attack_trace_point))
  (if (not (Variables|Default|GetisAttacking))
    (Variables|Default|SetisAttacking true)
    (Animation|Montage|PlayMontage (Variables|Character|GetMesh) "/Game/AI/Paired_PushShove_Att_Montage.Paired_PushShove_Att_Montage"
      (:then
        (bind (_outhit _returnvalue_2) (Collision|SphereTraceForObjects _returnvalue (+ _returnvalue (* (Math|Vector|GetForwardVector (Transformation|GetWorldRotation _attack_trace_point)) 7e+01)) 25.0 (Utilities|Array|MakeArray "ObjectTypeQuery3") false 0 "None"))
        (if _returnvalue_2
          (Game|Damage|ApplyDamage (.HitActor (Collision|BreakHitResult _outhit)) 1e+01 0 0)))
      (:OnCompleted
        (Variables|Default|SetisAttacking false)))))

(event Custom|Stop%20Seeing%20Player
  (AI|Components|Blackboard|SetValueasBool (AI|GetBlackboard (AI|GetAIController self)) (Utilities|Name|MakeLiteralName "SeePlayer") false)
  (Utilities|FlowControl|Delay 1.0)
  (if (not (ScalableFloat|GetValueasBool (AI|GetBlackboard (AI|GetAIController self)) (Utilities|Name|MakeLiteralName "SeePlayer")))
    (bind _chasing_music (Variables|Default|GetChasing%20Music)
      (:then
        (Audio|Components|Audio|FadeOut _chasing_music 3.0 0.0 "Linear" :!class /Script/Engine.AudioComponent))
      (:else))))

(event Game|Damage|EventAnyDamage
  (params (Damage :type Float%20%28single-precision%29) (DamageType :type Damage%20Type%20Object%20Reference) (InstigatedBy :type Controller%20Object%20Reference) (DamageCauser :type Actor%20Object%20Reference))
  (Physics|SetSimulatePhysics (Variables|Character|GetMesh) true)
  (Pawn|Components|CharacterMovement|SetMovementMode (Variables|Character|GetCharacterMovement) "MOVE_None" 0)
  (bind _returnvalue (UserInterface|CreateWidget "/Game/UI/WB_Win.WB_Win_C"))
  (UserInterface|Viewport|AddtoViewport _returnvalue 0)
  (Audio|PlaySoundatLocation "/Game/Audio/Grunt.Grunt" (Transformation|GetActorLocation) "0, 0, 0" 1.0 1.0 0.0 0 0 0 0)
  (Utilities|FlowControl|Delay 0.2)
  (Audio|PlaySound2D "/Game/Audio/Cinematic_Boom.Cinematic_Boom" 1.0 1.0 0.0 0 0))

(event EventBeginPlay
  (Utilities|Time|SetTimerbyEvent (delegate Custom|Stop%20Seeing%20Player) 0.8 true))

(fn ConstructionScript)